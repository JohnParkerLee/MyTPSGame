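; BP_Grenade is a grenade actor that explodes on a short fuse timer started at BeginPlay.
; Explode spawns the explosion particle, applies radial damage credited to its instigator, draws a debug sphere at the damage radius and fires a RadialForce impulse.
; The camera shake is centered on player 0's camera rather than the grenade, so distance from the blast does not weaken it.
; A second sequence branch spawns a smoke trail after the DestroyActor call.
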(event `self.ReceiveBeginPlay`
  (`KismetSystemLibrary.Delay` 1.5)
  (`self.Explode`))

(event `Explode`
  (bind _returnvalue (`self.K2_GetActorLocation`))
  (`|ExecutionSequence`
    (:`then_0`
      (`GameplayStatics.SpawnEmitterAtLocation` "/Game/WeaponEffects/Explosion/P_Explosion.P_Explosion" _returnvalue (struct) (2.0 2.0 2.0))
      (`GameplayStatics.ApplyRadialDamage` :`BaseDamage` 200.0 :`Origin` _returnvalue :`DamageRadius` (`self.Damage Radius`) :`DamageCauser` self :`InstigatedByController` (`self.GetInstigatorController`))
      (`KismetSystemLibrary.DrawDebugSphere` _returnvalue (`self.Damage Radius`) 12 (struct :`R` 1.0 :`G` 0.174713 :`B` 0.234453 :`A` 1.0) 1.0 2.0)
      (`GameplayStatics.PlayWorldCameraShake` "/Game/Blueprints/BP_Camerashake.BP_Camerashake_C" (`PlayerCameraManager.GetCameraLocation` (`GameplayStatics.GetPlayerCameraManager` 0)) 1.0 20.0)
      (`RadialForceComponent.FireImpulse` (`self.RadialForce`))
      (`self.K2_DestroyActor` self))
    (:`then_1`
      (`GameplayStatics.SpawnEmitterAtLocation` "/Game/WeaponEffects/BasicTracer/P_SmokeTrail.P_SmokeTrail" _returnvalue (struct) (2.0 2.0 2.0))
      (`self.SetLifeSpan` 0.0))))

(fn `UserConstructionScript`)