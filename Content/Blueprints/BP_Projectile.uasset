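; BP_Projectile is a projectile actor that leaves a bullet-mark decal where it hits and then destroys itself.
; On its first Hit, a DoOnce spawns a short-lived decal oriented to the surface normal, with fade screen size zeroed.
; An unconnected branch that would push physics-simulating components with a velocity-scaled impulse and draw a debug circle never runs.
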(event `self.ReceiveHit`
  (params (MyComp :type "PrimitiveComponent Object Reference") (Other :type "Actor Object Reference") (OtherComp :type "PrimitiveComponent Object Reference") (bSelfMoved :type Boolean) (HitLocation :type "Vector Structure") (HitNormal :type "Vector Structure") (NormalImpulse :type "Vector Structure") (Hit :type "HitResult Structure (by ref)"))
  (`|ExecutionSequence`
    (:`then_0`
      (`/Engine/EditorBlueprintResources/StandardMacros.DoOnce` false
        (:`Completed`
          (bind _returnvalue (`GameplayStatics.SpawnDecalAtLocation` "/Game/MP_bullet.MP_bullet" (20.0 20.0 20.0) HitLocation (`KismetMathLibrary.MakeRotFromX` HitNormal) 8.0))
          (`DecalComponent.SetFadeScreenSize` _returnvalue 0.0)
          (`self.K2_DestroyActor`))))))

(fn `UserConstructionScript`)